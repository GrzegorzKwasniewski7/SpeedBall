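; Player controller for a rolling-ball game that turns movement axis input into spin on the player's ball.
; It gets the ball from the first player's pawn through a GetBallRef message call and checks that it is valid.
; MoveForward applies torque around world Y and MoveHorizontal around X, both as acceleration changes so the ball's mass does not affect the response.
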(event Input|AxisEvents|InputAxisMoveForward
  (params (AxisValue :type Float%20%28single-precision%29))
  (bind _ball (Class|INTBPBall|GetBallRef(Message) (Game|Player|GetPlayerPawn 0)))
  (bind _ball_2 (Variables|/Game/Blueprints/BP_Ball.BP_Ball_C|GetBall _ball)
    (:then
      (Class|PrimitiveComponent|AddTorqueinRadians _ball_2 (Math|Vector|MakeVector 0.0 (* AxisValue 35.0) 0.0) "None" true))
    (:else)))

(event Input|AxisEvents|InputAxisMoveHorizontal
  (params (AxisValue :type Float%20%28single-precision%29))
  (bind _ball (Class|INTBPBall|GetBallRef(Message) (Game|Player|GetPlayerPawn 0)))
  (bind _ball_2 (Variables|/Game/Blueprints/BP_Ball.BP_Ball_C|GetBall _ball)
    (:then
      (Class|PrimitiveComponent|AddTorqueinRadians _ball_2 (Math|Vector|MakeVector (* AxisValue 35.0) 0.0 0.0) "None" true))
    (:else)))

(fn ConstructionScript)